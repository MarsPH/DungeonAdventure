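; BP_SpawnManager is a level spawner that places one skeleton enemy and one bow pickup on BeginPlay.
; SpawnEnemy picks a random X and Y within the SpawnArea component's bounds at a fixed SpawnHeight, ignoring its SpawnTransform input.
; SpawnPickup places the pickup at the RewardPos component's world location.
; Both functions take the class as a parameter and always spawn regardless of collision.
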(event `self.ReceiveBeginPlay`
  (`self.SpawnEnemy` "/Game/Blueprints/Characters/Skeleton/BP_Skeleton.BP_Skeleton_C" (`self.GetTransform`))
  (`self.SpawnPickup` "/Game/Blueprints/Pickups/BP_Pickup_Bow.BP_Pickup_Bow_C"))

(fn `SpawnEnemy`
  (params (Class :type "/Game/Blueprints/Characters/BP_Enemy_BASE Class Reference") (SpawnTransform :type "Transform Structure"))
  (locals (SpawnHeight :type "Float (double-precision)" :default 150.0))
  (bind (_origin _boxextent) (`KismetSystemLibrary.GetComponentBounds` (`self.SpawnArea`)))
  (bind (_returnvalue_x _returnvalue_y) (`KismetMathLibrary.BreakVector` (`KismetMathLibrary.RandomPointInBoundingBox` _origin _boxextent)))
  (`|SpawnActorFromClass` Class (`KismetMathLibrary.MakeTransform` (`KismetMathLibrary.MakeVector` _returnvalue_x _returnvalue_y (`local.SpawnHeight`))) "AlwaysSpawn" "MultiplyWithRoot" null null))

(fn `SpawnPickup`
  (params (Class :type "/Game/Blueprints/Pickups/BP_Pickup_BASE Class Reference"))
  (`|SpawnActorFromClass` Class (`KismetMathLibrary.MakeTransform` (`SceneComponent.K2_GetComponentLocation` (`self.RewardPos`))) "AlwaysSpawn" "MultiplyWithRoot" null null))

(fn `UserConstructionScript`)