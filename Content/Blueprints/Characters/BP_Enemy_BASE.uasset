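; Base enemy character that moves on request, damages BP_Hero on hurtbox overlap and reports its destruction to its owning spawner.
; It starts invincible with its hurtbox disabled and a looping flicker timer running.
; Hits trigger hit stop and a retriggerable stun that, like defeat, blocks movement.
; Defeat disables the hurtbox, then after a delay plays despawn sound, spawns skull-explosion VFX and destroys the actor.
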(event `self.ReceiveBeginPlay`
  (`parent.ReceiveBeginPlay`)
  (bind _returnvalue (`KismetSystemLibrary.K2_SetTimerDelegate` (`|CreateDelegate` :!event `SetSpriteVisiblity`) (`self.FlickerInterval`) true))
  (set `self.FlickerHandle` _returnvalue)
  (`PrimitiveComponent.SetCollisionEnabled` (`self.HurtBox`) "NoCollision")
  (`/Game/Blueprints/Components/BPC_Health.SetInvincibility` (`self.BPC_Health`)))

(event `WalkTowards`
  (params (Location :type "Vector Structure"))
  (if (and (not (`/Game/Blueprints/Components/BPC_Health.IsDefeated` (`self.BPC_Health`))) (not (`self.IsStunned`)))
    (`self.AddMovementInput` Location)))

(event `self.HurtBox.OnComponentBeginOverlap`
  (params (OverlappedComponent :type "PrimitiveComponent Object Reference") (OtherActor :type "Actor Object Reference") (OtherComp :type "PrimitiveComponent Object Reference") (OtherBodyIndex :type Integer) (bFromSweep :type Boolean) (SweepResult :type "HitResult Structure (by ref)"))
  (bind _asbp_hero (cast `/Game/Blueprints/Characters/Hero/BP_Hero` OtherActor))
  (if (== (`/Game/Blueprints/Characters/BP_Dungeon_Char_BASE.HurtBox` _asbp_hero) OtherComp)
    (`GameplayStatics.ApplyDamage` _asbp_hero 1.0 null self)))

(event `SetStun`
  (set `self.IsStunned` true)
  (`KismetSystemLibrary.RetriggerableDelay` (`self.StunDuration`))
  (set `self.IsStunned` false))

(event `HandleDefeat`
  (`PrimitiveComponent.SetCollisionEnabled` (`self.HurtBox`) "NoCollision")
  (`KismetSystemLibrary.Delay` (`self.DespawnDelay`))
  (`GameplayStatics.PlaySound2D` "/Game/Sounds/S_EnemyDespawn_Cue.S_EnemyDespawn_Cue" 1.0 1.0 0.0 null null)
  (`|SpawnActorFromClass` "/Game/Blueprints/VFX/BP_VFX_SkullExplostion.BP_VFX_SkullExplostion_C" (`KismetMathLibrary.MakeTransform` (`self.K2_GetActorLocation`)) "AlwaysSpawn" "MultiplyWithRoot" null null)
  (`self.K2_DestroyActor`))

(event `self.ReceiveDestroyed`
  (`/Game/Blueprints/Stystem/BP_SpawnManager.DefeatedEnemy` (`self.OwningSpawner`) self))

(fn `HandleHitExtended`
  (`self.HitStop`)
  (`self.SetStun`)
  (if (`/Game/Blueprints/Components/BPC_Health.IsDefeated` (`self.BPC_Health`))
    (`self.HandleDefeat`)))

(fn `UserConstructionScript`
  (`parent.UserConstructionScript`))