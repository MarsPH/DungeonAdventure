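; AI controller for BP_Enemy_BASE pawns that makes them chase the first player's pawn.
; It caches the enemy on possession and the target at BeginPlay, then checks their distance every tick.
; While beyond StopDistance, it passes the enemy's WalkTowards a straight-line look-at direction (despite the "Location" helper name), without navmesh pathfinding.
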(event `self.ReceivePossess`
  (params (PossessedPawn :type "Pawn Object Reference"))
  (bind _asbp_enemy_base (cast `/Game/Blueprints/Characters/BP_Enemy_BASE` PossessedPawn))
  (set `self.PossesedPawn` _asbp_enemy_base))

(event `self.ReceiveBeginPlay`
  (set `self.TargetPawn` (`GameplayStatics.GetPlayerPawn` 0)))

(event `self.ReceiveTick`
  (params (DeltaSeconds :type "Float (single-precision)"))
  (bind _targetpawn (`self.TargetPawn`)
    (:`then`
      (bind _returnvalue (`self.GetTargetDistance`))
      (if (> _returnvalue (`self.StopDistance`))
        (`/Game/Blueprints/Characters/BP_Enemy_BASE.WalkTowards` (`self.PossesedPawn`) (`self.GetWalkTowardsLocation` _targetpawn))))
    (:`else`)))

(fn `GetTargetDistance`
  (returns (ReturnValue :type "Float (double-precision)"))
  (return (`KismetMathLibrary.Vector_Distance` (`self.K2_GetActorLocation` (`self.TargetPawn`)) (`self.K2_GetActorLocation` (`self.PossesedPawn`)))))

(fn `GetWalkTowardsLocation`
  (params (TargetPawn :type "Actor Object Reference"))
  (returns (ReturnValue :type "Vector Structure"))
  (return (`KismetMathLibrary.GetForwardVector` (`KismetMathLibrary.FindLookAtRotation` (`self.K2_GetActorLocation` (`self.PossesedPawn`)) (`self.K2_GetActorLocation` TargetPawn)))))

(fn `UserConstructionScript`)